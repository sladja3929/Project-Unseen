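; BP_PatrolAIController is the AI controller for a patrolling enemy, feeding perception results into its Blackboard.
; On each target perception update it branches on the stimulus sense class.
; Sight stores an actor that casts to UnseenCharacter as TargetActor, while hearing stores the stimulus position as StimulusLocation.
; It does not check whether the stimulus was successfully sensed, so losing sight also writes TargetActor rather than clearing it.
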(event `self.AIPerception.OnTargetPerceptionUpdated`
  (params (Actor :type "Actor Object Reference") (Stimulus :type "AIStimulus Structure"))
  (bind _returnvalue (`AIPerceptionSystem.GetSenseClassForStimulus` Stimulus))
  (if (== _returnvalue "/Script/AIModule.AISense_Sight")
    (bind _asunseen_character (cast `UnseenCharacter` Actor))
    (`BlackboardComponent.SetValueAsObject` (`self.Blackboard`) "TargetActor" _asunseen_character)
    (elif (== _returnvalue "/Script/AIModule.AISense_Hearing")
      (`BlackboardComponent.SetValueAsVector` (`self.Blackboard`) "StimulusLocation" (`.StimulusLocation` (break `AIStimulus` Stimulus))))))

(fn `UserConstructionScript`
  (`parent.UserConstructionScript`))