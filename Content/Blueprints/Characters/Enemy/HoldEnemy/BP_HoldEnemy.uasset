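; BP_HoldEnemy is an enemy Blueprint whose AI is driven by Blackboard values for holding and monitoring locations.
; On BeginPlay it sets small detection and writes the DetectionState key.
; It then uses timed delays to set a hard-coded HoldLocation, set a MoniteringLocation and finally clear the latter, a scripted sequence that resembles test setup.
; Tick only calls the parent.
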(event `self.ReceiveBeginPlay`
  (`self.SetEnemyDetectionState` "SmallDetection")
  (`BlackboardComponent.SetValueAsEnum` (`AIBlueprintHelperLibrary.GetBlackboard` null) (`self.DetectionState`) 2)
  (`KismetSystemLibrary.Delay` 2.0)
  (`BlackboardComponent.SetValueAsVector` (`AIBlueprintHelperLibrary.GetBlackboard` null) (`self.HoldLocation`) (0.0 0.0 10.0))
  (`KismetSystemLibrary.Delay` 2.0)
  (`BlackboardComponent.SetValueAsVector` (`AIBlueprintHelperLibrary.GetBlackboard` null) (`self.MoniteringLocation`) (0.0 1000.0 10.0))
  (`KismetSystemLibrary.Delay` 2.0)
  (`BlackboardComponent.ClearValue` (`AIBlueprintHelperLibrary.GetBlackboard` null) (`self.MoniteringLocation`)))

(event `self.ReceiveTick`
  (params (DeltaSeconds :type "Float (single-precision)"))
  (`parent.ReceiveTick` DeltaSeconds))

(fn `UserConstructionScript`)