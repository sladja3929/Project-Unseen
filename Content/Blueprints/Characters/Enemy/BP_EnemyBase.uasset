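; Base enemy Blueprint that displays the enemy's detection state and combat gauge through its mesh and attached widgets.
; Each tick it reads the CombatGauge float from the Blackboard and pushes it to the combat gauge widget.
; When the detection state is set, it creates a dynamic material instance to tint the mesh and updates the head icon widget with the same color and an image.
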(event `self.ReceiveBeginPlay`)

(event `self.ReceiveTick`
  (params (DeltaSeconds :type "Float (single-precision)"))
  (bind _aswbp_combat_gauge_test (cast `/Game/Blueprints/UI/HeadIcon/WBP_CombatGaugeTest` (`WidgetComponent.GetWidget` (`self.CombatGaugeTest`))))
  (`/Game/Blueprints/UI/HeadIcon/WBP_CombatGaugeTest.UpdateCombatGauge` _aswbp_combat_gauge_test (`BlackboardComponent.GetValueAsFloat` (`AIBlueprintHelperLibrary.GetBlackboard` null) "CombatGauge")))

(event `self.EnemyDetectionStateSet`
  (bind _mesh (`self.Mesh`))
  (`|ExecutionSequence`
    (:`then_0`
      (bind _returnvalue (`PrimitiveComponent.CreateDynamicMaterialInstance` _mesh 0 (`PrimitiveComponent.GetMaterial` _mesh 0) "None"))
      (`MaterialInstanceDynamic.SetVectorParameterValue` _returnvalue "Tint" (`KismetMathLibrary.Conv_ColorToLinearColor` (`self.MaterialTintColor`)))
      (`PrimitiveComponent.SetMaterial` (`self.Mesh`) 0 _returnvalue))
    (:`then_1`
      (bind _aswbp_head_icon (cast `/Game/Blueprints/UI/HeadIcon/WBP_HeadIcon` (`WidgetComponent.GetWidget` (`self.HeadStateIcon`))))
      (`/Game/Blueprints/UI/HeadIcon/WBP_HeadIcon.UpdateIcon` _aswbp_head_icon (`KismetMathLibrary.Conv_ColorToLinearColor` (`self.MaterialTintColor`)) (`self.Image`)))))

(fn `UserConstructionScript`)